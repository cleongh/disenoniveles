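; Speed boost pickup that grants a player temporary super speed when taken.
; It overrides Taken, calls the parent version, then copies its SuperSpeedTime into the player's SuperSpeedActive and raises FloatingPawnMovement MaxSpeed to the player's SuperSpeedQuantity.
; The event graph and construction script add no logic, and nothing here counts down the boost or restores normal speed.
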(event EventBeginPlay
  (|CallParentFunction) ; This node is disabled and will not be called.\nDrag off pins to build functionality.
)

(event Collision|EventActorBeginOverlap
  (params (OtherActor :type Actor%20Object%20Reference))
  (|CallParentFunction OtherActor) ; This node is disabled and will not be called.\nDrag off pins to build functionality.
)

(event EventTick
  (params (DeltaSeconds :type Float%20%28single-precision%29))
  (|CallParentFunction DeltaSeconds) ; This node is disabled and will not be called.\nDrag off pins to build functionality.
)

(fn ConstructionScript
  (|CallParentFunction))

(fn Taken
  (params (Player :type Top%20Down%20Player%20Object%20Reference))
  (|CallParentFunction 0)
  (Variables|/Game/Blueprints/TopDownPlayer.TopDownPlayer_C|SetSuperSpeedActive Player (Variables|Game|GetSuper%20speed%20time))
  (Variables|/Script/Engine.FloatingPawnMovement|SetMaxSpeed (Variables|/Game/Blueprints/TopDownPlayer.TopDownPlayer_C|GetFloatingPawnMovement Player) (Variables|/Game/Blueprints/TopDownPlayer.TopDownPlayer_C|GetSuperSpeedQuantity Player)))