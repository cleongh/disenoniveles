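; Pickup actor that gives machine gun ammo to the player who takes it.
; Its Taken override calls the parent, then adds AmountBulletsUp to the player's Bullets map entry for one enum key (NewEnumerator1).
; The event graph holds only disabled default events, and the construction script just calls its parent.
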(event EventBeginPlay
  (|CallParentFunction) ; This node is disabled and will not be called.\nDrag off pins to build functionality.
)

(event Collision|EventActorBeginOverlap
  (params (OtherActor :type Actor%20Object%20Reference))
  (|CallParentFunction OtherActor) ; This node is disabled and will not be called.\nDrag off pins to build functionality.
)

(event EventTick
  (params (DeltaSeconds :type Float%20%28single-precision%29))
  (|CallParentFunction DeltaSeconds) ; This node is disabled and will not be called.\nDrag off pins to build functionality.
)

(fn ConstructionScript
  (|CallParentFunction))

(fn Taken
  (params (Player :type Top%20Down%20Player%20Object%20Reference))
  (bind _bullets (Variables|/Game/Blueprints/TopDownPlayer.TopDownPlayer_C|GetBullets Player))
  (|CallParentFunction Player)
  (Utilities|Map|Add _bullets "NewEnumerator1" (+ (.Value (Utilities|Map|Find _bullets "NewEnumerator1")) (Variables|Game|GetAmountBulletsUp))))